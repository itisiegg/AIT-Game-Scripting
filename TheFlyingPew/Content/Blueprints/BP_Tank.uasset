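; BP_Tank is a tank Blueprint that the player drives with W and S to move forward and back and A and D to rotate.
; Key press and release open and close four Gates, which a Sequence on Tick feeds into local offset and rotation calls.
; Movement is scaled by delta seconds for frame-rate independence and does not sweep for collision.
; The G key prints a test string.
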(event EventBeginPlay)

(event EventTick
  (params (DeltaSeconds :type Float%20%28single-precision%29))
  (Utilities|FlowControl|Sequence
    (:then_0
      (Utilities|FlowControl|Gate true
        (:Exit
          (Transformation|AddActorLocalOffset (* "100.000000,0.000000,0.000000" (Utilities|Time|GetWorldDeltaSeconds)) false false))))
    (:then_1
      (Utilities|FlowControl|Gate true
        (:Exit
          (Transformation|AddActorLocalOffset (* "-100.000000,0.000000,0.000000" (Utilities|Time|GetWorldDeltaSeconds)) false false))))
    (:then_2
      (Utilities|FlowControl|Gate true
        (:Exit
          (Transformation|AddActorLocalRotation (* "0.000000,-30.000000,0.000000" (Utilities|Time|GetWorldDeltaSeconds)) false false))))
    (:then_3
      (Utilities|FlowControl|Gate true
        (:Exit
          (Transformation|AddActorLocalRotation (* "0.000000,30.000000,0.000000" (Utilities|Time|GetWorldDeltaSeconds)) false false))))))

(event Input|KeyboardEvents|D
  (params (Key :type Key%20Structure :default "None"))
  (:Pressed
    (Utilities|FlowControl|Gate true) ; enters at Open
  )
  (:Released
    (Utilities|FlowControl|Gate true) ; enters at Close
  ))

(event Input|KeyboardEvents|G
  (params (Key :type Key%20Structure :default "None"))
  (:Pressed
    (Development|PrintString "Hello" true true "(R=0.000000,G=0.660000,B=1.000000,A=1.000000)" 4.0)))

(event Input|KeyboardEvents|W
  (params (Key :type Key%20Structure :default "None"))
  (:Pressed
    (Utilities|FlowControl|Gate true) ; enters at Open
  )
  (:Released
    (Utilities|FlowControl|Gate true) ; enters at Close
  ))

(event Input|KeyboardEvents|S
  (params (Key :type Key%20Structure :default "None"))
  (:Pressed
    (Utilities|FlowControl|Gate true) ; enters at Open
  )
  (:Released
    (Utilities|FlowControl|Gate true) ; enters at Close
  ))

(event Input|KeyboardEvents|A
  (params (Key :type Key%20Structure :default "None"))
  (:Pressed
    (Utilities|FlowControl|Gate true) ; enters at Open
  )
  (:Released
    (Utilities|FlowControl|Gate true) ; enters at Close
  ))

(fn ConstructionScript)