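; BP_Projectile is a projectile actor that damages whatever actor overlaps it and credits its shooter with score.
; On overlap it applies its Damage value, using the Instigator's controller as event instigator and the Instigator as damage causer, then destroys itself.
; If the Instigator is valid, it sends the damage amount to that PlayerState as score through an interface message.
; The construction script and GetPickUpStats are empty.
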(event Collision|EventActorBeginOverlap
  (params (OtherActor :type Actor%20Object%20Reference))
  ;[0.15 0.15 0.15 0.5] Applying Damage when in Radius
  (Game|Damage|ApplyDamage OtherActor (Variables|Default|GetDamage) (Pawn|GetController (Variables|Actor|GetInstigator)) (Variables|Actor|GetInstigator))
  (Utilities|FlowControl|Sequence
    (:then_1
      ;[0.15 0.15 0.15 0.5] Destroying Bullet
      (Actor|DestroyActor)
      (bind _instigator (Variables|Actor|GetInstigator)
        (:then
          ;[0.15 0.15 0.15 0.5] Adding to Score
          (Class|BPIMyFlyingGame|AddPlayerScore(Message) (Variables|/Script/Engine.Pawn|GetPlayerState _instigator) (Variables|Default|GetDamage)))
        (:else)))))

(fn ConstructionScript)

(fn GetPickUpStats
  (return ""))