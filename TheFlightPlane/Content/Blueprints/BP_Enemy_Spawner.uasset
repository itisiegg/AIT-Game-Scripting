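; Enemy spawner actor that continuously spawns random enemies along a line between two limit points.
; On BeginPlay a looping one-second timer fires the spawn event.
; Each spawn picks one of three enemy classes at random and places it at a random lerp between the left and right limit components, using the left limit's rotation.
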(event Custom|Spawn_EnemyA
  (Game|SpawnActorfromClass (Utilities|Array|Get(acopy) (Utilities|Array|MakeArray "/Game/Blueprints/BP_EnemyA.BP_EnemyA_C" "/Game/Blueprints/BP_EnemyB.BP_EnemyB_C" "/Game/Blueprints/BP_EnemyC.BP_EnemyC_C") (Math|Random|RandomInteger 3)) (Math|Transform|MakeTransform (Math|Vector|Lerp(Vector) (Transformation|GetWorldLocation (Variables|Default|GetLeftSpawnLimit1)) (Transformation|GetWorldLocation (Variables|Default|GetRightSpawnLimit)) (Math|Random|RandomFloat)) (Transformation|GetWorldRotation (Variables|Default|GetLeftSpawnLimit1)) "1.000000,1.000000,1.000000") "Undefined" "MultiplyWithRoot" 0 0))

(event EventBeginPlay
  (Utilities|Time|SetTimerbyEvent (delegate Custom|Spawn_EnemyA) 1.0 true))

(fn ConstructionScript)