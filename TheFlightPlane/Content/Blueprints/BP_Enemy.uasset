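; BP_Enemy is a damageable enemy that deals damage equal to its current Health to any actor overlapping its sphere.
; Incoming damage lowers Health, updates its widget with the health fraction and spawns a damage popup carrying the amount.
; A surviving hit plays a sound and temporarily applies an overlay material to the mesh, while zero Health plays a kill sound, spawns an explosion and destroys the actor.
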(event OnComponentBeginOverlap(Sphere)
  (params (OverlappedComponent :type Primitive%20Component%20Object%20Reference) (OtherActor :type Actor%20Object%20Reference) (OtherComp :type Primitive%20Component%20Object%20Reference) (OtherBodyIndex :type Integer) (bFromSweep :type Boolean) (SweepResult :type Hit%20Result%20Structure%20%28by%20ref%29))
  ;[0.15 0.15 0.15 0.5] Damage Recognizer
  (Game|Damage|ApplyDamage OtherActor (Variables|Default|GetHealth) 0 0))

(event Custom|HitSequence
  ;[0.15 0.15 0.15 0.5] Hit Sequence
  (Audio|PlaySound2D "/Game/Audio/MS_Hit.MS_Hit" 1.0 1.0 0.0 0 0)
  (Rendering|Material|SetOverlayMaterial (Variables|Default|GetStaticMesh) "/Game/Materials/M_Overlay.M_Overlay" :!class /Script/Engine.MeshComponent)
  (Utilities|FlowControl|Delay 2.0)
  (Rendering|Material|SetOverlayMaterial (Variables|Default|GetStaticMesh) 0 :!class /Script/Engine.MeshComponent))

(event Custom|KillSequence
  ;[0.15 0.15 0.15 0.5] Death Sequence
  (Audio|PlaySound2D "/Game/Audio/MS_Kill.MS_Kill" 1.0 1.0 0.0 0 0)
  (Game|SpawnActorfromClass "/Game/FX/BP_Explosion.BP_Explosion_C" (Math|Transform|MakeTransform (Transformation|GetActorLocation) "0, 0, 0" "1.000000,1.000000,1.000000") "AlwaysSpawn" "MultiplyWithRoot" 0 0)
  (Actor|DestroyActor))

(event Game|Damage|EventAnyDamage
  (params (Damage :type Float%20%28single-precision%29) (DamageType :type Damage%20Type%20Object%20Reference) (InstigatedBy :type Controller%20Object%20Reference) (DamageCauser :type Actor%20Object%20Reference))
  ;[0.15 0.15 0.15 0.5] Damage Calculator
  (Variables|Default|SetHealth (Math|Float|Max(Float) (- (Variables|Default|GetHealth) Damage) 0.0))
  (Utilities|FlowControl|Sequence
    (:then_0
      ;[0.15 0.15 0.15 0.5] Set Health
      (Class|BPIMyFlyingGame|SetHealth(Message) (UserInterface|GetUserWidgetObject (Variables|Default|GetWidget)) (Math|Float|SafeDivide (Variables|Default|GetHealth) (Variables|Default|GetMaxHealth))))
    (:then_1
      ;[0.15 0.15 0.15 0.5] Damage-Popup Appears
      (Game|SpawnActorfromClass "/Game/UI/BP_DamagePopUP.BP_DamagePopUP_C" (Math|Transform|MakeTransform (Transformation|GetActorLocation) "0, 0, 0" "1.000000,1.000000,1.000000") "Undefined" "MultiplyWithRoot" 0 Damage 0))
    (:then_2
      ;[0.15 0.15 0.15 0.5] Recognises if hit kills or not
      (if (== (Variables|Default|GetHealth) 0.0)
        (CallFunction|KillSequence)
        (else
          (CallFunction|HitSequence))))))

(fn ConstructionScript)