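; Enemy wave spawner that runs the waves defined in WavesData in order, then shows the WBP_End widget as a success.
; Each wave waits an initial delay, then repeatedly spawns its whole enemy list at timed intervals along a fixed X line, with random Y except on boss waves.
; A remaining count, set to the spawn count and decremented by destroy events, is polled after spawning to advance to the next wave.
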(event Custom|BeginSetOfWaves
  (Variables|Default|SetCurrentWaveIndex 0)
  (CallFunction|NextWave))

(event Custom|NextWave
  (if (> (Variables|Default|GetCurrentWaveIndex) (Variables|Default|GetLastWaveIndex))
    ;[0.15 0.15 0.15 0.5] Waves are Done
    (bind _returnvalue (UserInterface|CreateWidget "/Game/UI/WBP_End.WBP_End_C" (Game|GetPlayerController 0)))
    (UserInterface|Viewport|AddtoViewport _returnvalue 0)
    (else
      (Utilities|FlowControl|Delay (Utilities|Struct|BreakS_Waves (Utilities|Array|Get(acopy) (Variables|/Game/EnemyWaveSystem/PDA_Waves.PDA_Waves_C|GetWaves (Variables|Default|GetWavesData)) (Variables|Default|GetCurrentWaveIndex))))
      (CallFunction|BeginSpawn))))

(event Custom|NextSpawn
  (if (== (Variables|Default|GetCurrentSpawn) (Variables|Default|GetNumberToSpawn))
    (if (== (Variables|Default|GetEnemiesRemain) 0) :!label _label
      (Math|Integer|IncrementInt (Variables|Default|GetCurrentWaveIndex)
        (:%20%20
          (CallFunction|NextWave)))
      (else
        (Utilities|FlowControl|Delay 0.2)
        (goto _label)))
    (else
      (for _array_element (.enemies (Variables|Default|GetEnemiesToSpawn))
        (bind _returnvalue (Game|SpawnActorfromClass _array_element (Math|Transform|MakeTransform (Math|Vector|MakeVector 6.8e+03 (Math|Float|SelectFloat 0.0 (Math|Random|RandomFloatinRange -2e+03 2e+03) (.IsBossWave (Utilities|Struct|BreakS_Waves (Utilities|Array|Get(acopy) (Variables|/Game/EnemyWaveSystem/PDA_Waves.PDA_Waves_C|GetWaves (Variables|Default|GetWavesData)) (Variables|Default|GetCurrentWaveIndex))))) 0.0) "0.000000,180.000000,0.000000" "1.000000,1.000000,1.000000") "AlwaysSpawn" "MultiplyWithRoot" 0 0))
        (Game|BindEventtoOnDestroyed _returnvalue (delegate Custom|EnemyDestroyed)))
      (Math|Integer|IncrementInt (Variables|Default|GetCurrentSpawn)
        (:%20%20
          (Utilities|FlowControl|Delay (Variables|Default|GetTimeBetweenSpawn))
          (CallFunction|NextSpawn))))))

(event Custom|BeginSpawn
  (bind _wavesdata (Variables|Default|GetWavesData))
  (bind _currentwaveindex (Variables|Default|GetCurrentWaveIndex))
  (bind _waves (Variables|/Game/EnemyWaveSystem/PDA_Waves.PDA_Waves_C|GetWaves _wavesdata))
  (bind _output (Utilities|Array|Get(acopy) _waves _currentwaveindex))
  (bind (_timebetweenspawn _numberofspawns _enemies _isbosswave) (Utilities|Struct|BreakS_Waves _output))
  (Variables|Default|SetCurrentSpawn 0)
  (Variables|Default|SetTimeBetweenSpawn _timebetweenspawn)
  (bind _output_get (Variables|Default|SetNumberToSpawn _numberofspawns))
  (Variables|Default|SetEnemiesRemain _output_get)
  (Variables|Default|SetEnemiesToSpawn _enemies)
  (CallFunction|NextSpawn))

(event Custom|EnemyDestroyed
  (params (DestroyedActor :type Actor%20Object%20Reference))
  (Math|Integer|DecrementInt (Variables|Default|GetEnemiesRemain)))

(event EventBeginPlay
  (Variables|Default|SetLastWaveIndex (Utilities|Array|LastIndex (Variables|/Game/EnemyWaveSystem/PDA_Waves.PDA_Waves_C|GetWaves (Variables|Default|GetWavesData))))
  (CallFunction|BeginSetOfWaves))

(fn ConstructionScript)